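; Player controller that toggles two test UI widgets from hard-wired number keys.
; Key 1 flip-flops the custom inventory widget, giving it focus and showing the mouse cursor while open, then hiding the cursor on removal.
; Key 2 flip-flops the Countess skill-acquired widget without touching cursor or focus.
; Each widget is created on first use, cached in a variable and reused while valid.
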(event `Key|One`
  (params (Key :type "Key Structure"))
  (bind _testinventory (`self.TestInventory`))
  (:`Pressed`
    (`/Engine/EditorBlueprintResources/StandardMacros.FlipFlop`
      (:`A`
        (`/Engine/EditorBlueprintResources/StandardMacros.IsValid` _testinventory
          (:`Is Valid`
            (`UserWidget.AddToViewport` _testinventory 0)
            (set `self.bShowMouseCursor` true)
            (`Widget.SetFocus` (`self.TestInventory`)))
          (:`Is Not Valid`
            (bind _returnvalue (`|CreateWidget` "/Game/MyProjectMain/Blueprints/Test/UI/WBP_Inventory_Custom.WBP_Inventory_Custom_C"))
            (bind _output_get (set `self.TestInventory` _returnvalue))
            (`UserWidget.AddToViewport` _output_get 0)
            (`Widget.SetFocus` _output_get)
            (set `self.bShowMouseCursor` true))))
      (:`B`
        (`Widget.RemoveFromParent` _testinventory)
        (set `self.bShowMouseCursor` false)))))

(event `Key|Two`
  (params (Key :type "Key Structure"))
  (bind _testskillacquiredwidget (`self.TestSkillAcquiredWidget`))
  (:`Pressed`
    (`/Engine/EditorBlueprintResources/StandardMacros.FlipFlop`
      (:`A`
        (`/Engine/EditorBlueprintResources/StandardMacros.IsValid` _testskillacquiredwidget
          (:`Is Valid`
            (`UserWidget.AddToViewport` _testskillacquiredwidget 0))
          (:`Is Not Valid`
            (bind _returnvalue (`|CreateWidget` "/Game/MyProjectMain/Widgets/BP_Countess_Skill_Acquired_Widget.BP_Countess_Skill_Acquired_Widget_C"))
            (bind _output_get (set `self.TestSkillAcquiredWidget` _returnvalue))
            (`UserWidget.AddToViewport` _output_get 0))))
      (:`B`
        (`Widget.RemoveFromParent` _testskillacquiredwidget)))))

(fn `UserConstructionScript`)