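; Pickup actor for the Countess's Jump ability, named as a gameplay-ability granting actor; the grant logic itself is not in this graph.
; AbilityAcquiredEvent destroys the skill VFX, light and mesh through nested validity checks, then prints "Jump Acquired".
; A timeline that would lerp the mesh between begin and end positions is present but never runs.
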(event `self.AbilityAcquiredEvent`
  (bind _skill_mesh (`self.Skill_Mesh`))
  (bind _skill_vfx (`self.Skill_VFX`))
  (bind _skill_light (`self.Skill_Light`))
  (`/Engine/EditorBlueprintResources/StandardMacros.IsValid` _skill_vfx
    (:`Is Valid`
      (`ActorComponent.K2_DestroyComponent` _skill_vfx)
      (`/Engine/EditorBlueprintResources/StandardMacros.IsValid` _skill_light
        (:`Is Valid`
          (`ActorComponent.K2_DestroyComponent` _skill_light)
          (`/Engine/EditorBlueprintResources/StandardMacros.IsValid` _skill_mesh
            (:`Is Valid`
              (`ActorComponent.K2_DestroyComponent` _skill_mesh)
              (`KismetSystemLibrary.PrintString` "Jump Acquired"))))))))

(fn `UserConstructionScript`)